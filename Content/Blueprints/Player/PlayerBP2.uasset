(event Custom|moveMirrorAction_Event
  (bind _returnvalue (Transformation|GetActorLocation))
  (bind _returnvalue_2 (Transformation|GetActorForwardVector))
  (bind _hitactor (Variables|Default|GetHitActor))
  (bind _returnvalue_3 (* _returnvalue_2 1.2e+02))
  (bind _returnvalue_4 (* _returnvalue_2 6e+01))
  (bind _returnvalue_5 (+ _returnvalue _returnvalue_3))
  (bind _returnvalue_6 (+ _returnvalue _returnvalue_4))
  (bind _floatobj (Timeline|Float Play)
    (:Update
      (bind _returnvalue_7 (Collision|BoxTraceByChannel _returnvalue_6 _returnvalue_6 "100.000000,60.000000,60.000000" (Math|Rotator|FindLookatRotation _returnvalue _returnvalue_5) "TraceTypeQuery1" false (Utilities|Array|MakeArray (Variables|Default|GetHitActor)) "ForOneFrame"))
      (if (not _returnvalue_7)
        (Transformation|SetActorLocation _hitactor (Math|Interpolation|VInterpTo (Transformation|GetActorLocation _hitactor) _returnvalue_5 (stale EventTick DeltaSeconds) 2e+01) false false)
        (Transformation|AddActorLocalOffset _hitactor (Math|Vector|MakeVector 0.0 0.0 (* _floatobj 1e+01)) false false)))))

(event Custom|mirrorAction_イベント_0
  (bind _returnvalue (Transformation|GetActorRotation))
  (bind _hitactor (Variables|Default|GetHitActor))
  (bind (_roll _pitch) (Math|Rotator|BreakRotator _returnvalue))
  ;[1 1 1] ミラーアクション
  (Transformation|SetActorRotation (Math|Rotator|MakeRotator _roll _pitch (.Yaw (Math|Rotator|BreakRotator (Math|Interpolation|RInterpTo _returnvalue (Math|Rotator|FindLookatRotation (Transformation|GetActorLocation) (Transformation|GetActorLocation (Variables|Default|GetHitActor))) (stale EventTick DeltaSeconds) 1.0)))))
  (キャラクター|LightBulbOff)
  (if (Variables|Default|GetRight_Rot)
    (Transformation|AddActorLocalRotation _hitactor "0,1.000000, 0" true false)
    (elif (Variables|Default|GetLeft_Rot)
      (Transformation|AddActorLocalRotation _hitactor "0,-1.000000, 0" true false)
      (elif (Variables|Default|GetUp_Rot)
        (Transformation|AddActorLocalRotation _hitactor "-1.000000,0.000000,0.000000" true false)
        (elif (Variables|Default|GetDown_Rot)
          (Transformation|AddActorLocalRotation _hitactor "1.000000,0.000000,0.000000" true false))))))

(event EventBeginPlay
  (EventDispatchers|AssignMirrorAction (delegate Custom|mirrorAction_イベント_0))
  (EventDispatchers|BindEventtoMoveMirrorAction (delegate Custom|moveMirrorAction_Event)))

(event EventTick
  (params (DeltaSeconds :type Float%20%28single-precision%29))
  (bind _returnvalue (Transformation|GetActorLocation))
  (bind _returnvalue_2 (Transformation|GetActorForwardVector))
  (bind _hitactor (Variables|Default|GetHitActor))
  (bind _returnvalue_3 (* _returnvalue_2 1.2e+02))
  (bind _returnvalue_4 (* _returnvalue_2 6e+01))
  (bind _returnvalue_5 (+ _returnvalue _returnvalue_3))
  (bind _returnvalue_6 (+ _returnvalue _returnvalue_4))
  ;[1 1 1] 電球をカメラの方向にする
  (Transformation|SetWorldRotation (Variables|Default|GetLightBulb) (Math|Rotator|MakeRotator 0.0 0.0 (.yaw (Math|Rotator|FindLookatRotation (Transformation|GetActorLocation) (Transformation|GetActorLocation (Game|GetPlayerCameraManager 0))))) false false)
  ;[1 1 1] アクション関連
  (bind _hitactor_2 (キャラクター|Investigate))
  (bind _newparam (キャラクター|Tag _hitactor_2))
  (if _newparam
    (キャラクター|LightBulbon)
    (else
      (キャラクター|LightBulbOff)))
  (if (Variables|Default|GetActionFlg)
    (Default|CallMirrorAction)
    (elif (Variables|Default|GetCarryFlg)
      (Default|CallMoveMirrorAction)
      (else
        (bind _floatobj (Timeline|Float Stop)
          (:Update
            (bind _returnvalue_7 (Collision|BoxTraceByChannel _returnvalue_6 _returnvalue_6 "100.000000,60.000000,60.000000" (Math|Rotator|FindLookatRotation _returnvalue _returnvalue_5) "TraceTypeQuery1" false (Utilities|Array|MakeArray (Variables|Default|GetHitActor)) "ForOneFrame"))
            (if (not _returnvalue_7)
              (Transformation|SetActorLocation _hitactor (Math|Interpolation|VInterpTo (Transformation|GetActorLocation _hitactor) _returnvalue_5 DeltaSeconds 2e+01) false false)
              (Transformation|AddActorLocalOffset _hitactor (Math|Vector|MakeVector 0.0 0.0 (* _floatobj 1e+01)) false false))))))))

(event Input|AxisEvents|InputAxisMoveForward
  (params (AxisValue :type Float%20%28single-precision%29))
  ;[1 1 1] 移動
  (if (not (Variables|Default|GetActionFlg))
    (Pawn|Input|AddMovementInput (Transformation|GetActorForwardVector (Game|GetPlayerCameraManager 0)) AxisValue false) ; 前後移動
  ))

(event Input|AxisEvents|InputAxisMoveRight
  (params (AxisValue :type Float%20%28single-precision%29))
  ;[1 1 1] 移動
  (if (not (Variables|Default|GetActionFlg))
    (Pawn|Input|AddMovementInput (Transformation|GetActorRightVector (Game|GetPlayerCameraManager 0)) AxisValue false) ; 左右移動
  ))

(event Input|KeyboardEvents|Right
  (params (Key :type Key%20Structure))
  ;[1 1 1] ミラーアクション
  (:Pressed
    (Variables|Default|SetRight_Rot true))
  (:Released
    (Variables|Default|SetRight_Rot false)))

(event Input|KeyboardEvents|SpaceBar
  (params (Key :type Key%20Structure))
  ;[1 1 1] ジャンプ
  (:Pressed
    (if (not (Variables|Default|GetActionFlg))
      (if (not (Variables|Default|GetCarryFlg))
        (Character|Jump))))
  (:Released
    (Character|StopJumping)))

(event Input|KeyboardEvents|X
  (params (Key :type Key%20Structure))
  ;[1 1 1] アクション関連
  (:Pressed
    (if (not (Variables|Default|GetActionFlg))
      (bind _hitactor (キャラクター|Investigate))
      (if (キャラクター|IsMoveMirror _hitactor)
        (bind _output_get (Variables|Default|SetHitActor _hitactor))
        (bind _newparam (キャラクター|Tag _output_get))
        (if _newparam
          (Utilities|FlowControl|FlipFlop
            (:A
              (Variables|Default|SetCarryFlg true))
            (:B
              (Variables|Default|SetCarryFlg false :!label _label)
              (Transformation|SetActorLocation _output_get (Math|Vector|MakeVector (.X (Math|Vector|BreakVector (Transformation|GetActorLocation _output_get))) (.Y (Math|Vector|BreakVector (Transformation|GetActorLocation _output_get))) (Variables|Default|GetUpBase)) false false)))
          (else
            (goto _label)))))))

(event Input|KeyboardEvents|Z
  (params (Key :type Key%20Structure))
  ;[1 1 1] アクション関連
  (:Pressed
    (if (not (Variables|Default|GetCarryFlg))
      (bind _hitactor (キャラクター|Investigate))
      (bind _output_get (Variables|Default|SetHitActor _hitactor))
      (bind _newparam (キャラクター|Tag _output_get))
      (if _newparam
        (Utilities|FlowControl|FlipFlop
          (:A
            (Variables|Default|SetActionFlg true))
          (:B
            (Variables|Default|SetActionFlg false :!label _label)))
        (else
          (goto _label))))))

(event Input|KeyboardEvents|D
  (params (Key :type Key%20Structure))
  ;[1 1 1] ミラーアクション
  (:Pressed
    (Variables|Default|SetRight_Rot true))
  (:Released
    (Variables|Default|SetRight_Rot false)))

(event Input|KeyboardEvents|A
  (params (Key :type Key%20Structure))
  ;[1 1 1] ミラーアクション
  (:Pressed
    (Variables|Default|SetLeft_Rot true))
  (:Released
    (Variables|Default|SetLeft_Rot false)))

(event Input|KeyboardEvents|S
  (params (Key :type Key%20Structure))
  ;[1 1 1] ミラーアクション
  (:Pressed
    (Variables|Default|SetDown_Rot true))
  (:Released
    (Variables|Default|SetDown_Rot false)))

(event Input|KeyboardEvents|Left
  (params (Key :type Key%20Structure))
  ;[1 1 1] ミラーアクション
  (:Pressed
    (Variables|Default|SetLeft_Rot true))
  (:Released
    (Variables|Default|SetLeft_Rot false)))

(event Input|KeyboardEvents|Up
  (params (Key :type Key%20Structure))
  ;[1 1 1] ミラーアクション
  (:Pressed
    (Variables|Default|SetUp_Rot true))
  (:Released
    (Variables|Default|SetUp_Rot false)))

(event Input|KeyboardEvents|Down
  (params (Key :type Key%20Structure))
  ;[1 1 1] ミラーアクション
  (:Pressed
    (Variables|Default|SetDown_Rot true))
  (:Released
    (Variables|Default|SetDown_Rot false)))

(event Input|KeyboardEvents|W
  (params (Key :type Key%20Structure))
  ;[1 1 1] ミラーアクション
  (:Pressed
    (Variables|Default|SetUp_Rot true))
  (:Released
    (Variables|Default|SetUp_Rot false)))

(fn ConstructionScript
  (bind _returnvalue (Rendering|Material|CreateDynamicMaterialInstance (Variables|Character|GetMesh) 2 "/Game/Blueprints/Player/Material/M_Rook_Eye_Inst.M_Rook_Eye_Inst" "None" :!class /Script/Engine.PrimitiveComponent))
  (Rendering|Material|SetVectorParameterValue _returnvalue "LightColor" (Variables|Default|GetLightColor) :!class /Script/Engine.MaterialInstanceDynamic)
  (Rendering|Material|SetScalarParameterValue _returnvalue "LightPow" (Variables|Default|GetLightPow) :!class /Script/Engine.MaterialInstanceDynamic)
  (Variables|Default|SetUpBase 2e+01))

(fn Investigate
  (bind _returnvalue (Transformation|GetActorLocation))
  (bind _returnvalue_2 (Transformation|GetActorForwardVector))
  (bind _returnvalue_3 (* _returnvalue_2 5e+01))
  (bind _returnvalue_4 (+ _returnvalue _returnvalue_3))
  (bind _outhit (Collision|BoxTraceByChannel _returnvalue_4 _returnvalue_4 "50.000000,60.000000,50.000000" (Transformation|GetWorldRotation (Variables|Character|GetMesh)) "TraceTypeQuery1" false 0 "None"))
  (return (.HitActor (Collision|BreakHitResult _outhit))))

(fn Tag
  (params (Actor :type Actor%20Object%20Reference))
  (if (Utilities|IsValid Actor)
    (return (Actor|ActorHasTag Actor (GameplayTags|GetTagName (GameplayTags|MakeLiteralGameplayTag))))
    (else
      (return false))))

(fn LightBulbon
  (bind _lightbulb (Variables|Default|GetLightBulb))
  (Rendering|SetVisibility _lightbulb true false)
  (Development|SetHiddeninGame _lightbulb false false)
  (return))

(fn LightBulbOff
  (bind _lightbulb (Variables|Default|GetLightBulb))
  (Rendering|SetVisibility _lightbulb false false)
  (Development|SetHiddeninGame _lightbulb true false)
  (return))

(fn IsMoveMirror
  (params (ActorRef :type Actor%20Object%20Reference))
  (bind _tags (Variables|/Script/Engine.Actor|GetTags ActorRef))
  (if (Utilities|IsValid ActorRef)
    (if (== (Utilities|Array|Length _tags) 2)
      (if (and (Utilities|Name|Equal(Name) (Utilities|Array|Get(acopy) _tags) "Mirror") (Utilities|Name|Equal(Name) (Utilities|Array|Get(acopy) _tags 1) "Move"))
        (return true)
        (else
          (return false))))))