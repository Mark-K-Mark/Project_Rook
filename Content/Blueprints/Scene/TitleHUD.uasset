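; Title screen HUD that shows a full-screen title image and launches Reflection_Map when Enter is pressed.
; BeginPlay forces a 640x480 resolution through a console command and enables input on the HUD.
; Enter sets IsLoading, so DrawHUD layers the full-screen Start texture over the title.
; It then calls a non-blocking, hidden LoadStreamLevel on the map before switching to it with OpenLevel.
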(event EventBeginPlay
  (Development|ExecuteConsoleCommand (Utilities|String|Append "r.setRes" (Utilities|String|Append (Utilities|String|Append "640" "x") "480")) 0)
  (Input|EnableInput 0))

(event Collision|EventActorBeginOverlap
  (params (OtherActor :type Actor%20Object%20Reference)))

(event EventTick
  (params (DeltaSeconds :type Float%20%28single-precision%29)))

(event EventDrawHUD
  (params (SizeX :type Integer) (SizeY :type Integer))
  (bind _returnvalue (Viewport|GetViewportSize))
  (bind (_x _y) (Math|Vector2D|BreakVector2D _returnvalue))
  (Canvas|DrawTexture "/Game/Architecture/Textures/Title1.Title1" 0.0 0.0 _x _y 0.0 0.0 1.0 1.0 "(R=1.000000,G=1.000000,B=1.000000,A=1.000000)")
  (if (Variables|Default|GetIsLoading)
    (Canvas|DrawTexture "/Game/Architecture/Textures/Start.Start" 0.0 0.0 _x _y 0.0 0.0 1.0 1.0 "(R=1.000000,G=1.000000,B=1.000000,A=1.000000)")))

(event Input|KeyboardEvents|Enter
  (params (Key :type Key%20Structure))
  (:Pressed
    (Variables|Default|SetIsLoading true)
    (Game|LoadStreamLevel(byName) "Reflection_Map" false)
    (Game|OpenLevel(byName) "Reflection_Map")))

(fn ConstructionScript)