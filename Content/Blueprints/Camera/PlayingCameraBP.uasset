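; PlayingCameraBP is a gameplay camera actor that becomes the player's view target on BeginPlay and follows the player pawn.
; The construction script records its starting position and the Floor actor's X bounds extent.
; Each tick it interpolates between that start and an EndPoint actor using pawn X divided by the extent, unclamped.
; It also rotates to look at the pawn.
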(event EventBeginPlay
  (Game|Player|SetViewTargetwithBlend (Game|GetPlayerController 0) self 0.0 "VTBlend_Linear" 0.0 false))

(event EventTick
  (params (DeltaSeconds :type Float%20%28single-precision%29))
  (bind _returnvalue (Game|Player|GetPlayerPawn 0))
  (bind _returnvalue_2 (Transformation|GetActorLocation _returnvalue))
  (Transformation|SetActorLocationAndRotation (Math|Vector|Lerp(Vector) (Variables|Default|GetStartPos) (Transformation|GetActorLocation (Variables|Default|GetEndPoint)) (/ (.X (Math|Vector|BreakVector _returnvalue_2)) (Variables|Default|GetFloorWidth))) (Math|Rotator|FindLookatRotation (Transformation|GetActorLocation) _returnvalue_2)))

(fn ConstructionScript
  (bind _output_get (Variables|Default|SetStartPos (Transformation|GetActorLocation)))
  (Variables|Default|SetFloorWidth (.X (Math|Vector|BreakVector (.BoxExtent (Collision|GetActorBounds (Variables|Default|GetFloor) false)))))
  (Variables|Default|SetEndPos _output_get))