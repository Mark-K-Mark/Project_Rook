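; SplineCameraBP is a camera actor that becomes the player's view on BeginPlay and travels along a spline.
; Each tick, the player pawn's X offset from the starting controller position, wrapped by a Floor-derived width, becomes a looping spline distance.
; The local spline point is added to the construction-time origin, and the camera aims below its Target actor.
; A time-based MoveDistance accumulates but never drives movement.
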(event EventBeginPlay
  (bind _returnvalue (Game|GetPlayerController 0))
  (Variables|Default|SetStartCharaPos (Transformation|GetActorLocation _returnvalue))
  (Game|Player|SetViewTargetwithBlend _returnvalue self 0.0 "VTBlend_Linear" 0.0 false))

(event EventTick
  (params (DeltaSeconds :type Float%20%28single-precision%29))
  (Transformation|SetActorRotation (Math|Rotator|FindLookatRotation (Transformation|GetActorLocation) (+ (Transformation|GetActorLocation (Variables|Default|GetTarget)) "0, 0,-1000.000000")))
  (Variables|Default|SetMoveDistance (+ (* DeltaSeconds 1e+02) (Variables|Default|GetMoveDistance)))
  (bind _location (CallFunction|GetCurrentLocation (Math|Float|%(Float) (- (.X (Math|Vector|BreakVector (Transformation|GetActorLocation (Game|Player|GetPlayerPawn 0)))) (.X (Math|Vector|BreakVector (Variables|Default|GetStartCharaPos)))) (* (.X (Math|Vector|BreakVector (.BoxExtent (Collision|GetActorBounds (Variables|Default|GetFloor) false)))) 1.7)) true))
  (Transformation|SetActorLocation (+ _location (Variables|Default|GetStartPos)) false false))

(fn ConstructionScript
  (Variables|Default|SetStartPos (Transformation|GetActorLocation)))

(fn GetCurrentLocation
  (params (Length :type Float%20%28single-precision%29) (Loop :type Boolean))
  (bind _spline (Variables|Default|GetSpline))
  (if Loop
    (Variables|Default|SetLocalLength (Math|Float|%(Float) Length (Spline|GetSplineLength _spline)))
    (return (Spline|GetLocationatDistanceAlongSpline _spline (Variables|Default|GetLocalLength) "Local"))
    (else
      (Variables|Default|SetLocalLength Length))))

(fn GetSplineLength
  (return (Spline|GetSplineLength (Variables|Default|GetSpline))))