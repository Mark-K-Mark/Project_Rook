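; LightSource is an actor that casts a sight line forward and can sweep its facing back and forth.
; Each tick it runs a 500-unit visibility line trace with persistent debug drawing and calls the HitNow dispatcher when something blocks it.
; A separate Hit event steps local yaw one degree per call, toggling direction at the 0 and -90 degree limits.
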(event EventBeginPlay)

(event Collision|EventActorBeginOverlap
  (params (OtherActor :type Actor%20Object%20Reference)))

(event EventTick
  (params (DeltaSeconds :type Float%20%28single-precision%29))
  (bind _returnvalue (Transformation|GetActorLocation))
  (bind (_outhit _returnvalue_2) (Collision|LineTraceByChannel _returnvalue (+ _returnvalue (* (Transformation|GetActorForwardVector) 500)) "TraceTypeQuery1" false 0 "Persistent"))
  (if _returnvalue_2
    (Default|CallHitNow)))

(event Collision|EventHit
  (params (MyComp :type Primitive%20Component%20Object%20Reference) (Other :type Actor%20Object%20Reference) (OtherComp :type Primitive%20Component%20Object%20Reference) (bSelfMoved :type Boolean) (HitLocation :type Vector :default "0, 0, 0") (HitNormal :type Vector :default "0, 0, 0") (NormalImpulse :type Vector :default "0, 0, 0") (Hit :type Hit%20Result%20Structure%20%28by%20ref%29))
  (bind _returnvalue (Transformation|GetActorRotation))
  (bind _yaw (Math|Rotator|BreakRotator _returnvalue))
  (if (>= _yaw 0.0)
    (Variables|Default|SetLeftRot (not (Variables|Default|GetLeftRot))))
  (if (<= _yaw -9e+01)
    (Variables|Default|SetLeftRot (not (Variables|Default|GetLeftRot))))
  (if (Variables|Default|GetLeftRot)
    (Transformation|AddActorLocalRotation "0.000000,-1.000000, 0" false false)
    (else
      (Transformation|AddActorLocalRotation "0.000000,1.000000, 0" false false))))

(fn ConstructionScript)