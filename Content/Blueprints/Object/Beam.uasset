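; Beam actor that fires a straight light ray along its particle component's forward vector, apparently for a mirror-reflection light puzzle.
; ShotAction line-traces on Visibility up to MaxLength and sets the particle beam's endpoints to the start and the impact or maximum point.
; Hits on "Mirror" or "Clear" tagged actors only return a Loop flag; reflection data is unused.
; Tick's call sits in a while loop with a false condition, so it never runs.
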(event EventBeginPlay
  (Variables|Default|SetShot true))

(event Collision|EventActorBeginOverlap
  (params (OtherActor :type Actor%20Object%20Reference)))

(event EventTick
  (params (DeltaSeconds :type Float%20%28single-precision%29))
  (bind _beam (Variables|Default|GetBeam))
  (bind _returnvalue (Transformation|GetWorldLocation _beam))
  (while false
    (bind _hitinfo (CallFunction|ShotAction _returnvalue (+ _returnvalue (* (Math|Vector|GetForwardVector _beam) (Variables|Default|GetMaxLength)))))))

(fn ConstructionScript
  (Variables|Default|SetMaxLength 5e+03)
  (Variables|Default|SetSpeed 1e+03)
  (Variables|Default|SetNowLength 0.0)
  (Variables|Default|SetTime 0.0))

(fn ShotAction
  (params (LightStart :type Vector) (LightEnd :type Vector))
  (bind _beam (Variables|Default|GetBeam))
  (bind _beam_2 (Variables|Default|GetBeam))
  ;[1 1 1] 光の線の表示・非表示処理
  (if (Components|Activation|IsActive _beam)
    _
    (else
      (Components|Activation|Activate _beam false) ; 光の線を表示
    ))
  (bind (_outhit _returnvalue) (Collision|LineTraceByChannel LightStart LightEnd "TraceTypeQuery1" false 0 "None")) ; 光の線を発射
  (if _returnvalue
    (Class|ParticleSystemComponent|SetBeamTargetPoint _beam_2 0 (.ImpactPoint (Collision|BreakHitResult _outhit))) ; 当たった場所が終点
    (else
      (Variables|Default|SetTime 0.0)
      (Class|ParticleSystemComponent|SetBeamTargetPoint _beam_2 0 LightEnd) ; 上限の長さまで伸ばす
    ))
  (Class|ParticleSystemComponent|SetBeamSourcePoint _beam_2 0 LightStart) ; パーティクル開始位置
  (if (Utilities|IsValid (.HitActor (Collision|BreakHitResult _outhit)))
    (Utilities|FlowControl|Sequence
      (:then_0
        ;[1 1 1] HitReflectionの呼び出し元
        (if (Actor|ActorHasTag (.HitActor (Collision|BreakHitResult _outhit)) "Mirror")
          (return true "")))
      (:then_1
        ;[1 1 1] HitClearの呼び出し元
        (if (Actor|ActorHasTag (.HitActor (Collision|BreakHitResult _outhit)) "Clear")
          (return false ""))))))

(fn GetSpeed
  (return (Variables|Default|GetSpeed)))

(fn GetMaxLength
  (return (Variables|Default|GetMaxLength)))