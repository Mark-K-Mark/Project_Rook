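; ReflectionObj is an actor tagged "Mirror" in its construction script that rotates in yaw when its Hit event fires.
; Each Hit turns it one degree in the direction set by LeftRot, which flips at limits measured from the rotation saved at BeginPlay.
; Both limit checks resolve to start yaw plus 90, because the lower one subtracts a negative, so the intended two-sided sweep is not symmetric.
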(event EventBeginPlay
  (Variables|Default|SetDefaultRot (Transformation|GetActorRotation)))

(event Collision|EventActorBeginOverlap
  (params (OtherActor :type Actor%20Object%20Reference)))

(event EventTick
  (params (DeltaSeconds :type Float%20%28single-precision%29)))

(event Collision|EventHit
  (params (MyComp :type Primitive%20Component%20Object%20Reference) (Other :type Actor%20Object%20Reference) (OtherComp :type Primitive%20Component%20Object%20Reference) (bSelfMoved :type Boolean) (HitLocation :type Vector :default "0, 0, 0") (HitNormal :type Vector :default "0, 0, 0") (NormalImpulse :type Vector :default "0, 0, 0") (Hit :type Hit%20Result%20Structure%20%28by%20ref%29))
  (bind _returnvalue (Transformation|GetActorRotation))
  (bind _defaultrot (Variables|Default|GetDefaultRot))
  (bind _yaw (Math|Rotator|BreakRotator _defaultrot))
  (bind _yaw_2 (Math|Rotator|BreakRotator _returnvalue))
  (if (Variables|Default|GetLeftRot)
    (Transformation|AddActorLocalRotation "0,1.000000, 0" false false)
    (if (>= _yaw_2 (+ _yaw 9e+01))
      (Variables|Default|SetLeftRot (not (Variables|Default|GetLeftRot))))
    (else
      (Transformation|AddActorLocalRotation "0,-1.000000, 0" false false)
      (if (<= _yaw_2 (- _yaw -9e+01))
        (Variables|Default|SetLeftRot (not (Variables|Default|GetLeftRot)))))))

(fn ConstructionScript
  (|CallParentFunction)
  (Variables|Default|SetTags (Utilities|Array|MakeArray "Mirror")))

(fn GetTagName
  (return "None"))