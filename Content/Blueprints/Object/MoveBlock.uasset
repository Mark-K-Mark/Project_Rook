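; MoveBlock is a switch-triggered block that slides back and forth between two positions.
; The construction script sets the endpoints from the Cube's location and a point 100 units along its forward vector.
; A PlayerBP2 hit on the Switch component flips the direction and starts a move, unless one is already running.
; Tick lerps the Cube by a fixed step per frame, so speed depends on frame rate.
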(event Custom|OnComponentHit_イベント_0
  (params (HitComponent :type Primitive%20Component%20Object%20Reference) (OtherActor :type Actor%20Object%20Reference) (OtherComp :type Primitive%20Component%20Object%20Reference) (NormalImpulse :type Vector) (Hit :type Hit%20Result%20Structure%20%28by%20ref%29))
  (if (== (Utilities|GetClass OtherActor) "/Game/Blueprints/Player/PlayerBP2.PlayerBP2_C")
    (if (not (Variables|Default|GetMove))
      (Variables|Default|SetIsFront (not (Variables|Default|GetIsFront)))
      (Variables|Default|SetMove true)
      (Variables|Default|SetLerpCnt 0.0))))

(event EventTick
  (params (DeltaSeconds :type Float%20%28single-precision%29))
  (if (Variables|Default|GetMove)
    (if (Variables|Default|GetIsFront)
      (if (<= (Variables|Default|GetLerpCnt) 1.0)
        (Transformation|SetWorldLocation (Variables|Default|GetCube) (Math|Vector|Lerp(Vector) (Variables|Default|GetStartPos) (Variables|Default|GetEndPos) (Variables|Default|GetLerpCnt)) false false)
        (Variables|Default|SetLerpCnt (+ (Variables|Default|GetLerpCnt) 0.01))
        (else
          (Variables|Default|SetMove false)))
      (elif (<= (Variables|Default|GetLerpCnt) 1.0)
        (Transformation|SetWorldLocation (Variables|Default|GetCube) (Math|Vector|Lerp(Vector) (Variables|Default|GetEndPos) (Variables|Default|GetStartPos) (Variables|Default|GetLerpCnt)) false false)
        (Variables|Default|SetLerpCnt (+ (Variables|Default|GetLerpCnt) 0.01))
        (else
          (Variables|Default|SetMove false))))))

(event EventBeginPlay
  (Collision|AssignOnComponentHit (Variables|Default|GetSwitch) (delegate Custom|OnComponentHit_イベント_0)))

(fn ConstructionScript
  (bind _cube (Variables|Default|GetCube))
  (bind _returnvalue (Transformation|GetWorldLocation _cube))
  (Variables|Default|SetMove false)
  (Variables|Default|SetStartPos _returnvalue)
  (Variables|Default|SetEndPos (+ _returnvalue (* (Math|Vector|GetForwardVector _cube) 100)))
  (Variables|Default|SetIsFront false))